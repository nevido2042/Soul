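; BP_Castle_Guard is a player-controlled guard character that attaches weapon and shield child actors to mesh sockets on BeginPlay.
; Input drives montage-gated jumping and toggles or switches targets through a lock-on component.
; Falling polls vertical speed to flag hard landings, which play a montage and disable movement until it ends.
; Sword combo, roll and walk/run speed-blending logic exists but is not wired to any event.
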(event Custom|Check%20Speed
  ;[1 1 1] Hard Land
  (if (Utilities|Enum|Equal(Enum) (stale EventOnMovementModeChanged NewMovementMode) "MOVE_Falling")
    (if (<= (.z (Transformation|GetVelocity)) -1e+03)
      (Variables|Default|SetbHardLanding true)
      (else
        (Utilities|FlowControl|Delay 0.2)
        (CallFunction|CheckSpeed)))))

(event Input|EnhancedActionEvents|EnhancedInputActionIA_Run
  (params (ActionValue :type Boolean) (ElapsedSeconds :type Float%20%28double-precision%29) (TriggeredSeconds :type Float%20%28double-precision%29) (InputAction :type Input%20Action%20Object%20Reference :default "/Game/My/Actors/Controller/Input/IA_Run.IA_Run"))
  ;[1 1 1] 걷기/달리기
)

(event Input|EnhancedActionEvents|EnhancedInputActionIA_TargetLockOn
  (params (ActionValue :type Boolean) (ElapsedSeconds :type Float%20%28double-precision%29) (TriggeredSeconds :type Float%20%28double-precision%29) (InputAction :type Input%20Action%20Object%20Reference :default "/Game/My/Actors/Controller/Input/IA_TargetLockOn.IA_TargetLockOn"))
  (bind _bp_targetlockoncomponent (Variables|Default|GetBP_TargetLockOnComponent))
  ;[1 1 1] 타겟 락 온
  (if (Variables|/Game/My/Components/BP_TargetLockOnComponent.BP_TargetLockOnComponent_C|GetLockOn _bp_targetlockoncomponent)
    (Default|StopTargetLockon _bp_targetlockoncomponent)
    (else
      (Default|TriggerTargetLockon (Variables|Default|GetBP_TargetLockOnComponent)))))

(event EventBeginPlay
  (bind _weapon (Variables|Default|GetWeapon))
  (bind _shield (Variables|Default|GetShield))
  (bind _mesh (Variables|Character|GetMesh))
  (bind _mesh_2 (Variables|Character|GetMesh))
  (bind _childactor (Variables|/Script/Engine.ChildActorComponent|GetChildActor _weapon))
  (bind _childactor_2 (Variables|/Script/Engine.ChildActorComponent|GetChildActor _shield))
  (Utilities|FlowControl|Sequence
    (:then_0
      ;[1 1 1] 방패 붙이기
      (Transformation|AttachComponentToComponent _childactor _mesh_2 (Class|SkinnedMeshComponent|GetSocketBoneName _mesh_2 "WeaponSocket") "KeepRelative" "KeepRelative" "KeepRelative" false)
      (Transformation|SetActorRelativeTransform _childactor (Math|Transform|MakeTransform "-6.313255,-19.926998,8.154418" "-25.451300,89.195738,81.288308" "1.000000,1.000000,1.000000") false false))
    (:then_1
      ;[1 1 1] 무기 붙이기
      (Transformation|AttachComponentToComponent _childactor_2 _mesh (Class|SkinnedMeshComponent|GetSocketBoneName _mesh "ShieldSocket") "KeepRelative" "KeepRelative" "KeepRelative" false)
      (Transformation|SetActorRelativeTransform _childactor_2 (Math|Transform|MakeTransform "-0.899504,-5.941859,-8.912465" "-15.082850,87.031459,86.673784" "1.000000,1.000000,1.000000") false false))))

(event EventOnMovementModeChanged
  (params (PrevMovementMode :type EMovementMode%20Enum :default "MOVE_None") (NewMovementMode :type EMovementMode%20Enum :default "MOVE_None") (PrevCustomMode :type Byte :default 0) (NewCustomMode :type Byte :default 0))
  (bind _charactermovement (Variables|Character|GetCharacterMovement))
  ;[1 1 1] Hard Land
  (Utilities|FlowControl|Sequence
    (:then_0
      (if (Utilities|Enum|Equal(Enum) NewMovementMode "MOVE_Falling")
        (if (<= (.z (Transformation|GetVelocity)) -1e+03)
          (Variables|Default|SetbHardLanding true)
          (else
            (Utilities|FlowControl|Delay 0.2)
            (CallFunction|CheckSpeed)))))
    (:then_1
      (if (and (Utilities|Enum|Equal(Enum) NewMovementMode "MOVE_Walking") (Variables|Default|GetbHardLanding))
        (Pawn|Components|CharacterMovement|DisableMovement _charactermovement)
        (bind _returnvalue (Animation|PlayAnimMontage "/Game/Castle_Guard_RootBone/Animations/HardLanding_UE_Montage.HardLanding_UE_Montage" 1.0 "None"))
        (Variables|Default|SetbHardLanding false)
        (Utilities|FlowControl|Delay _returnvalue)
        (Pawn|Components|CharacterMovement|SetMovementMode _charactermovement "MOVE_Walking" 0)))))

(event EventTick
  (params (DeltaSeconds :type Float%20%28single-precision%29))
  ;[1 1 1] 걷기/달리기
)

(event Input|MouseEvents|LeftMouseButton
  (params (Key :type Key%20Structure :default "None"))
  ;[1 1 1] 연속공격
)

(event Input|KeyboardEvents|SpaceBar
  (params (Key :type Key%20Structure :default "None"))
  ;[1 1 1] 구르기
)

(event Input|MouseEvents|MouseWheelDown
  (params (Key :type Key%20Structure :default "None"))
  ;[1 1 1] 타겟 락 온
  (:Pressed
    (Default|SwitchTargetonRight (Variables|Default|GetBP_TargetLockOnComponent))))

(event Input|KeyboardEvents|F
  (params (Key :type Key%20Structure :default "None"))
  ;[1 1 1] 점프
  (:Pressed
    (if (not (Class|AnimInstance|IsAnyMontagePlaying (Components|SkeletalMesh|GetAnimInstance (Variables|Character|GetMesh))))
      (Character|Jump))))

(event Input|MouseEvents|MouseWheelUp
  (params (Key :type Key%20Structure :default "None"))
  ;[1 1 1] 타겟 락 온
  (:Pressed
    (Default|SwtichTargetonLeft (Variables|Default|GetBP_TargetLockOnComponent))))

(fn ConstructionScript)

(fn Run
  (Variables|Default|SetbRun true)
  (Variables|/Script/Engine.CharacterMovementComponent|SetMaxWalkSpeed (Variables|Character|GetCharacterMovement) (Math|Float|Lerp (Variables|/Script/Engine.CharacterMovementComponent|GetMaxWalkSpeed (Variables|Character|GetCharacterMovement)) (Variables|Default|GetRunSpeed_0) (* (Utilities|Time|GetWorldDeltaSeconds) 3.0))))

(fn Walk
  (Variables|Default|SetbRun false)
  (Variables|/Script/Engine.CharacterMovementComponent|SetMaxWalkSpeed (Variables|Character|GetCharacterMovement) (Math|Float|Lerp (Variables|/Script/Engine.CharacterMovementComponent|GetMaxWalkSpeed (Variables|Character|GetCharacterMovement)) (Variables|Default|GetWalkSpeed_0) (* (Utilities|Time|GetWorldDeltaSeconds) 3.0))))

(fn GetCamera
  (return (Variables|Default|GetCamera)))